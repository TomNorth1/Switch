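; Battery-powered door actor that rises vertically when opened, at a cost in the player's batteries.
; OpenDoor asks the player's BP_ParallelCharacter to remove BatteryCost batteries, printing a message if that fails.
; On success, a timeline adds its Z track to the start location saved at BeginPlay.
; IsOpen is set only when the timeline finishes, blocking later opens; the door has no closing logic.
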(event EventBeginPlay
  (Variables|Default|SetStartLocation (Transformation|GetWorldLocation (Variables|Transformation|GetRootComponent))))

(event Collision|EventActorBeginOverlap
  (params (OtherActor :type Actor%20Object%20Reference)))

(event EventTick
  (params (DeltaSeconds :type Float%20%28single-precision%29)))

(event EventOpenDoor
  (bind _returnvalue (Game|Player|GetPlayerPawn 0))
  (bind _startlocation (Variables|Default|GetStartLocation))
  (if (not (Variables|Default|GetbIsOpen))
    (if (Utilities|IsValid _returnvalue)
      (bind _asbp_parallel_character (Utilities|Casting|CastToBP_ParallelCharacter _returnvalue))
      (bind _returnvalue_2 (Class|ParallelCharacter|RemoveBattery _asbp_parallel_character (Variables|Default|GetBatteryCost)))
      (if _returnvalue_2
        (bind _z (Timeline|Timeline_0 Play)
          (:Update
            (Transformation|SetWorldLocation (Variables|Transformation|GetRootComponent) (Math|Vector|MakeVector (.x _startlocation) (.y _startlocation) (+ (.z _startlocation) _z)) false false))
          (:Finished
            (Variables|Default|SetbIsOpen true)))
        (else
          (Development|PrintString "Not Enough Batteries"))))))

(fn ConstructionScript)