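; BP_Checkpoint is a checkpoint trigger that updates the spawn location when a BP_ParallelCharacter overlaps its Box.
; It writes its own transform to SpawnLocation on BP_ParallelGameModeBase when its BlueWorld flag is set.
; Otherwise it shifts the location by a hardcoded negative Y offset, so the saved spawn apparently always maps to the blue world's side of the parallel layout.
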(event OnComponentBeginOverlap(Box)
  (params (OverlappedComponent :type Primitive%20Component%20Object%20Reference) (OtherActor :type Actor%20Object%20Reference) (OtherComp :type Primitive%20Component%20Object%20Reference) (OtherBodyIndex :type Integer) (bFromSweep :type Boolean) (SweepResult :type Hit%20Result%20Structure%20%28by%20ref%29))
  (bind _self self)
  (bind _returnvalue (Transformation|GetActorTransform _self))
  (bind (_location _rotation _scale) (Math|Transform|BreakTransform _returnvalue))
  (Utilities|Casting|CastToBP_ParallelCharacter OtherActor)
  (bind _asbp_parallel_game_mode_base (Utilities|Casting|CastToBP_ParallelGameModeBase (Game|GetGameMode)))
  (if (Variables|Default|GetBlueWorld)
    (Variables|/Game/Blueprints/BP_ParallelGameModeBase.BP_ParallelGameModeBase_C|SetSpawnLocation _asbp_parallel_game_mode_base _returnvalue)
    (else
      (Variables|/Game/Blueprints/BP_ParallelGameModeBase.BP_ParallelGameModeBase_C|SetSpawnLocation _asbp_parallel_game_mode_base (Math|Transform|MakeTransform (Math|Vector|MakeVector (.x _location) (- (.y _location) 2.2e+04) (.z _location)) _rotation _scale)))))

(event EventBeginPlay)

(event Collision|EventActorBeginOverlap
  (params (OtherActor :type Actor%20Object%20Reference)))

(event EventTick
  (params (DeltaSeconds :type Float%20%28single-precision%29)))

(fn ConstructionScript)