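; BP_Enemy is a battery-powered turret enemy that fires projectiles after spotting the player's BP_ParallelCharacter.
; PawnSensing sets FoundPlayer, so Tick eases the Arrow toward the player and otherwise back to its starting rotation.
; Delays inside Tick pace the shot, spawning BP_EnemyProjectile at the Scene component with zero rotation before clearing the flag.
; Without a valid BPBattery child actor, the PowerDown timeline rolls the head mesh instead.
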(event OnSeePawn(PawnSensing)
  (params (Pawn :type Pawn%20Object%20Reference))
  (Utilities|Casting|CastToBP_ParallelCharacter Pawn)
  (Variables|Default|SetFoundPlayer true))

(event EventBeginPlay
  (Variables|Default|SetStartRotation (Transformation|GetWorldRotation (Variables|Default|GetArrow))))

(event Collision|EventActorBeginOverlap
  (params (OtherActor :type Actor%20Object%20Reference)))

(event EventTick
  (params (DeltaSeconds :type Float%20%28single-precision%29))
  (bind _returnvalue (Game|Player|GetPlayerPawn 0))
  (bind _arrow (Variables|Default|GetArrow))
  (bind _sm_enemyhead (Variables|Default|GetSM_EnemyHead))
  (bind _returnvalue_2 (Transformation|GetWorldRotation _sm_enemyhead))
  (if (Utilities|IsValid (Variables|/Script/Engine.ChildActorComponent|GetChildActor (Variables|Default|GetBP_Battery)))
    (if (Variables|Default|GetFoundPlayer)
      (if (Utilities|IsValid _returnvalue)
        (Transformation|SetWorldRotation _arrow (Math|Interpolation|RInterpTo (Transformation|GetWorldRotation _arrow) (Math|Rotator|FindLookatRotation (Transformation|GetActorLocation) (Transformation|GetActorLocation _returnvalue)) DeltaSeconds 5.0) false false)
        (Utilities|FlowControl|Delay 2.5)
        (Game|SpawnActorfromClass "/Game/Blueprints/BP_EnemyProjectile.BP_EnemyProjectile_C" (Math|Transform|MakeTransform (Transformation|GetWorldLocation (Variables|Default|GetScene))) "Undefined" 0 0)
        (Utilities|FlowControl|Delay 0.2)
        (Variables|Default|SetFoundPlayer false))
      (else
        (Transformation|SetWorldRotation _arrow (Math|Interpolation|RInterpTo (Transformation|GetWorldRotation (Variables|Default|GetArrow)) (Variables|Default|GetStartRotation) DeltaSeconds 12.0) false false)))
    (else
      (bind _rot (Timeline|PowerDown Play)
        (:Update
          (Transformation|SetWorldRotation _sm_enemyhead (Math|Rotator|MakeRotator _rot (.pitch _returnvalue_2) (.yaw _returnvalue_2)) false false))))))

(fn ConstructionScript)