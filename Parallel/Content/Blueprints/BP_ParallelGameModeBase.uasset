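; Game mode for the Parallel game that handles player death and respawn while keeping collected batteries.
; On BeginPlay and respawn, it puts the character in the blue world, restores its battery count and binds to its destruction.
; When destroyed, it records the batteries, adds a death on the player controller, fades the camera out, then spawns and possesses a new character at SpawnLocation before fading back in.
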(event Custom|PlayerDied
  (params (DestroyedActor :type Actor%20Object%20Reference))
  (bind _returnvalue (Game|GetPlayerController 0))
  (bind _playercameramanager (Variables|/Script/Engine.PlayerController|GetPlayerCameraManager _returnvalue))
  (bind _asbp_parallel_player_controller (Utilities|Casting|CastToBP_ParallelPlayerController _returnvalue))
  (Default|AddDeath _asbp_parallel_player_controller)
  (bind _asbp_parallel_character (Utilities|Casting|CastToBP_ParallelCharacter DestroyedActor))
  (bind _output_get (Variables|Default|SetNum%20Of%20Batteries%20At%20Death (Variables|/Script/Parallel.ParallelCharacter|GetNumOfBatteries _asbp_parallel_character)))
  (CameraFades|StartCameraFade :self _playercameramanager :ToAlpha 1.0 :Duration 1.0 :bHoldWhenFinished true)
  (Utilities|FlowControl|Delay 1.0)
  (bind _returnvalue_2 (Game|SpawnActorfromClass "/Game/Blueprints/BP_ParallelCharacter.BP_ParallelCharacter_C" (Variables|Default|GetSpawnLocation) "Undefined" 0 0))
  (CameraFades|StartCameraFade :self _playercameramanager :FromAlpha 1.0 :Duration 1.0)
  (Pawn|Possess _returnvalue _returnvalue_2)
  (CallFunction|Respawn))

(event Custom|Respawn
  (bind _asbp_parallel_character (Utilities|Casting|CastToBP_ParallelCharacter (Game|GetPlayerCharacter 0)))
  (Variables|/Script/Parallel.ParallelCharacter|SetbBlueWorld _asbp_parallel_character true)
  (while (> (stale Custom|PlayerDied _output_get) (Variables|/Script/Parallel.ParallelCharacter|GetNumOfBatteries _asbp_parallel_character))
    (Class|ParallelCharacter|AddBattery _asbp_parallel_character))
  (Game|BindEventtoOnDestroyed _asbp_parallel_character (delegate Custom|PlayerDied)))

(event EventBeginPlay
  (bind _asbp_parallel_character (Utilities|Casting|CastToBP_ParallelCharacter (Game|GetPlayerCharacter 0)))
  (Variables|/Script/Parallel.ParallelCharacter|SetbBlueWorld _asbp_parallel_character true)
  (while (> (stale Custom|PlayerDied _output_get) (Variables|/Script/Parallel.ParallelCharacter|GetNumOfBatteries _asbp_parallel_character))
    (Class|ParallelCharacter|AddBattery _asbp_parallel_character))
  (Game|BindEventtoOnDestroyed _asbp_parallel_character (delegate Custom|PlayerDied)))

(event EventTick
  (params (DeltaSeconds :type Float%20%28single-precision%29)))

(fn ConstructionScript)