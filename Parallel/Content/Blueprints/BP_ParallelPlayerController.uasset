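; BP_ParallelPlayerController is the player controller that tracks deaths and switches and presents the end-game screen.
; AddDeath and AddSwitch each increment a counter.
; EndGame sets GameOver, adds a WBP_EndGame widget with both tallies and game time, and shows the mouse cursor.
; The widget's tallies are wired from the increment nodes' outputs in those other events, rather than from variable reads.
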(event Custom|EndGame
  (Variables|Default|SetGameOver true)
  (bind _returnvalue (UserInterface|CreateWidget "/Game/Blueprints/WBP_EndGame.WBP_EndGame_C" 0 (stale Custom|AddDeath _result) (stale Custom|AddSwitch _result) (Utilities|Time|GetTimeSeconds)))
  (UserInterface|Viewport|AddtoViewport _returnvalue 0)
  (Variables|Default|SetbShowMouseCursor true))

(event Custom|AddDeath
  (bind _result (Math|Integer|IncrementInt (Variables|Default|GetNumberOfDeaths))))

(event Custom|AddSwitch
  (bind _result (Math|Integer|IncrementInt (Variables|Default|GetNumberOfSwitches))))

(event EventBeginPlay)

(event EventTick
  (params (DeltaSeconds :type Float%20%28single-precision%29)))

(fn ConstructionScript)