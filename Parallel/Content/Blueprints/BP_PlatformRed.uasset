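; BP_PlatformRed is a falling platform that shakes when stepped on, drops, then resets.
; Its Box overlap responds only to BP_ParallelCharacter and plays the Rumble timeline, which offsets the Cube's height from the cached start location.
; When the timeline finishes, the Cube falls under physics and gravity.
; After a short delay, physics is switched off and the Cube returns to the transform saved at BeginPlay.
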(event OnComponentBeginOverlap(Box)
  (params (OverlappedComponent :type Primitive%20Component%20Object%20Reference) (OtherActor :type Actor%20Object%20Reference) (OtherComp :type Primitive%20Component%20Object%20Reference) (OtherBodyIndex :type Integer) (bFromSweep :type Boolean) (SweepResult :type Hit%20Result%20Structure%20%28by%20ref%29))
  (bind _startlocation (Variables|Default|GetStartLocation))
  (bind _cube (Variables|Default|GetCube))
  (Utilities|Casting|CastToBP_ParallelCharacter OtherActor)
  (bind _newtrack_0 (Timeline|Rumble PlayFromStart)
    (:Update
      (Transformation|SetWorldLocation (Variables|Default|GetCube) (Math|Vector|MakeVector (.x _startlocation) (.y _startlocation) (+ (.z _startlocation) _newtrack_0)) false false))
    (:Finished
      (Physics|SetSimulatePhysics (Variables|Default|GetCube) true)
      (Physics|SetEnableGravity _cube true)
      (Utilities|FlowControl|Delay 2.0)
      (Physics|SetSimulatePhysics _cube false)
      (Physics|SetEnableGravity _cube false)
      (Transformation|SetWorldTransform (Variables|Default|GetCube) (Variables|Default|GetStartTransformation) false false))))

(event EventBeginPlay
  (Variables|Default|SetStartLocation (Transformation|GetWorldLocation (Variables|Default|GetDefaultSceneRoot)))
  (Variables|Default|SetStartTransformation (Transformation|GetWorldTransform (Variables|Default|GetCube))))

(event Collision|EventActorBeginOverlap
  (params (OtherActor :type Actor%20Object%20Reference)))

(event EventTick
  (params (DeltaSeconds :type Float%20%28single-precision%29)))

(fn ConstructionScript)