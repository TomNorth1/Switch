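; BP_WeightDoor is a two-panel puzzle door that opens when all four referenced triggers report Triggered.
; Tick polls the triggers and calls OpenDoor while all are active, which clears Locked and plays a timeline.
; The timeline offsets the blue and red door meshes along world Z from start positions cached at BeginPlay.
; The graph has no closing or relocking logic.
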(event Custom|OpenDoor
  (Variables|Default|SetLocked false)
  (bind _newtrack_2 (Timeline|Timeline_0 Play)
    (:Update
      (Transformation|SetWorldLocation (Variables|Default|GetSM_DoorBlue) (+ (Variables|Default|GetStartLocationBlue) (Math|Vector|MakeVector 0.0 0.0 _newtrack_2)) false false)
      (Transformation|SetWorldLocation (Variables|Default|GetSM_DoorRed) (+ (Variables|Default|GetStartLocationRed) (Math|Vector|MakeVector 0.0 0.0 _newtrack_2)) false false))))

(event EventBeginPlay
  (Variables|Default|SetLocked true)
  (Variables|Default|SetStartLocationBlue (Transformation|GetWorldLocation (Variables|Default|GetSM_DoorBlue)))
  (Variables|Default|SetStartLocationRed (Transformation|GetWorldLocation (Variables|Default|GetSM_DoorRed))))

(event Collision|EventActorBeginOverlap
  (params (OtherActor :type Actor%20Object%20Reference)))

(event EventTick
  (params (DeltaSeconds :type Float%20%28single-precision%29))
  (if (Variables|/Game/Blueprints/BP_DoorTrigger.BP_DoorTrigger_C|GetTriggered (Variables|Default|GetTrigger1))
    (if (Variables|/Game/Blueprints/BP_DoorTrigger.BP_DoorTrigger_C|GetTriggered (Variables|Default|GetTrigger2))
      (if (Variables|/Game/Blueprints/BP_DoorTrigger.BP_DoorTrigger_C|GetTriggered (Variables|Default|GetTrigger3))
        (if (Variables|/Game/Blueprints/BP_DoorTrigger.BP_DoorTrigger_C|GetTriggered (Variables|Default|GetTrigger4))
          (CallFunction|OpenDoor))))))

(fn ConstructionScript)